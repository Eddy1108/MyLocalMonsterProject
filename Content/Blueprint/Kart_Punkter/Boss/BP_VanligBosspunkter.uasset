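; Regular boss point on the map that opens a battle when clicked.
; Clicking its Plane creates the Blob_Battle widget and adds it to the viewport, while hovering switches the mouse cursor to a hand.
; Tick adds a world rotation to the flipbook from a delta-scaled Z vector converted to a rotator, which discards magnitude, so the step does not scale with frame time.
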(event OnClicked(Plane)
  (params (TouchedComponent :type Primitive%20Component%20Object%20Reference) (ButtonPressed :type Key%20Structure :default "None"))
  (bind _returnvalue (UserInterface|CreateWidget "/Game/UI/Slime_Battle/Blob_Battle.Blob_Battle_C"))
  (UserInterface|Viewport|AddtoViewport _returnvalue 0))

(event OnBeginCursorOver(Plane)
  (params (TouchedComponent :type Primitive%20Component%20Object%20Reference))
  (Variables|/Script/Engine.PlayerController|SetCurrentMouseCursor (Game|GetPlayerController 0) "Hand"))

(event OnEndCursorOver(Plane)
  (params (TouchedComponent :type Primitive%20Component%20Object%20Reference))
  (Variables|/Script/Engine.PlayerController|SetCurrentMouseCursor (Game|GetPlayerController 0) "Default"))

(event EventBeginPlay)

(event EventTick
  (params (DeltaSeconds :type Float%20%28single-precision%29))
  (Transformation|AddWorldRotation (Variables|Default|GetFlipbookComponent) (Math|Conversions|RotationFromXVector (* "0, 0,2.000000" (Utilities|Time|GetWorldDeltaSeconds))) false false))

(fn ConstructionScript)