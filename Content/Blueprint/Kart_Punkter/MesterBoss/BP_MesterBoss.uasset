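; BP_MesterBoss is a clickable, pulsing boss marker that opens the first boss question.
; Tick oscillates the actor's X and Z scale between two limits, holding Y at zero.
; Hovering the Cone component switches the mouse cursor to a hand.
; Clicking it creates the Boss_Question1 widget only if the monster game mode flags Moth, Cat, Scream and Blob all complete.
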(event OnClicked(Cone)
  (params (TouchedComponent :type Primitive%20Component%20Object%20Reference) (ButtonPressed :type Key%20Structure :default "None"))
  (CallFunction|CompleteCheck))

(event OnBeginCursorOver(Cone)
  (params (TouchedComponent :type Primitive%20Component%20Object%20Reference))
  (Variables|/Script/Engine.PlayerController|SetCurrentMouseCursor (Game|GetPlayerController 0) "Hand"))

(event OnEndCursorOver(Cone)
  (params (TouchedComponent :type Primitive%20Component%20Object%20Reference))
  (Variables|/Script/Engine.PlayerController|SetCurrentMouseCursor (Game|GetPlayerController 0) "Default"))

(event EventBeginPlay
  (Variables|Default|SetScale 0.15)
  (bind _asbp_my_local_monster_game_mode_base (Utilities|Casting|CastToBP_MyLocalMonsterGameModeBase (Game|GetGameMode)))
  (Variables|Default|SetMonsterGMRef _asbp_my_local_monster_game_mode_base))

(event Collision|EventActorBeginOverlap
  (params (OtherActor :type Actor%20Object%20Reference)))

(event EventTick
  (params (DeltaSeconds :type Float%20%28single-precision%29))
  (CallFunction|ExclamationRotate DeltaSeconds))

(fn ConstructionScript)

(fn ExclamationRotate
  (params (DeltaTime :type Float%20%28single-precision%29))
  (Variables|Default|SetDeltaTime DeltaTime)
  (if (> (Variables|Default|GetScale) 0.15)
    (Variables|Default|SetDirection false))
  (if (< (Variables|Default|GetScale) 0.12)
    (Variables|Default|SetDirection true))
  (if (Variables|Default|GetDirection)
    (Transformation|SetActorScale3D (Math|Vector|MakeVector (Variables|Default|GetScale) 0.0 (Variables|Default|GetScale)))
    (Variables|Default|SetScale (+ (Variables|Default|GetScale) (* (Variables|Default|GetDeltaTime) 0.04)))
    (else
      (Transformation|SetActorScale3D (Math|Vector|MakeVector (Variables|Default|GetScale) 0.0 (Variables|Default|GetScale)))
      (Variables|Default|SetScale (+ (Variables|Default|GetScale) (* (Variables|Default|GetDeltaTime) -0.04))))))

(fn CompleteCheck
  (bind _monstergmref (Variables|Default|GetMonsterGMRef))
  (if (Variables|/Game/Blueprint/BP_MyLocalMonsterGameModeBase.BP_MyLocalMonsterGameModeBase_C|GetcompleteMoth _monstergmref)
    (if (Variables|/Game/Blueprint/BP_MyLocalMonsterGameModeBase.BP_MyLocalMonsterGameModeBase_C|GetcompleteCat _monstergmref)
      (if (Variables|/Game/Blueprint/BP_MyLocalMonsterGameModeBase.BP_MyLocalMonsterGameModeBase_C|GetcompleteScream _monstergmref)
        (if (Variables|/Game/Blueprint/BP_MyLocalMonsterGameModeBase.BP_MyLocalMonsterGameModeBase_C|GetcompleteBlob _monstergmref)
          (bind _returnvalue (UserInterface|CreateWidget "/Game/UI/Boss_Battle/Boss_Question1.Boss_Question1_C"))
          (UserInterface|Viewport|AddtoViewport _returnvalue 0))))))