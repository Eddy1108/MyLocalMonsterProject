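; BP_Test_HUD is a test Blueprint that exercises the monster avatar and opens the start menu.
; On BeginPlay it finds the BP_MonsterAvatar in the level, applies hard-coded body, face and head changes, then calls PrintTests.
; It then creates the Start_Meny widget and adds it to the viewport.
; An unconnected node chain for setting a portrait screen resolution never runs.
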(event EventBeginPlay
  (bind _returnvalue (Actor|GetActorOfClass "/Game/Blueprint/BP_MonsterAvatar.BP_MonsterAvatar_C"))
  (bind _output_get (Variables|Default|SetMonsterAvatar _returnvalue))
  (Class|MonsterAvatar|ChangeBody _output_get 4.0)
  (Class|MonsterAvatar|ChangeFace _output_get 1.0)
  (Class|MonsterAvatar|ChangeHead _output_get 2.0)
  (Class|TestHUD|PrintTests)
  (bind _returnvalue_2 (UserInterface|CreateWidget "/Game/UI/Start_Meny.Start_Meny_C"))
  (UserInterface|Viewport|AddtoViewport _returnvalue_2 0))

(event Collision|EventActorBeginOverlap
  (params (OtherActor :type Actor%20Object%20Reference)))

(event EventTick
  (params (DeltaSeconds :type Float%20%28single-precision%29)))

(fn ConstructionScript)